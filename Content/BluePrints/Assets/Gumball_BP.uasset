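; Gumball machine actor that opens a color customization widget when the player interacts with it.
; GumballBox overlap with ThirdPersonCharacter toggles actor input, so E works only in range.
; Pressing E disables input, shows the widget with UI-only input and cursor, hides the player, then plays a timed machine animation and sound.
; Camera zoom and E-prompt widget logic is left unconnected.
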(event `self.ReceiveBeginPlay`
  (bind _output_get (set `self.e_WD REF` (`self.e_WD REF`)))
  (set `self.e_WD REF` _output_get))

(event `Key|E`
  (params (Key :type "Key Structure"))
  (bind _returnvalue (`GameplayStatics.GetPlayerController` 0))
  ;[0 0 0] Camera zoom in to shop when on trigger (VideoPart1)
  (:`Pressed`
    (`self.DisableInput` null)
    (bind _returnvalue_2 (`|CreateWidget` "/Game/BluePrints/UI/GumballMachineColorCustom_WD.gumballMachineColorCustom_WD_C"))
    (`UserWidget.AddToViewport` _returnvalue_2 0)
    (`WidgetBlueprintLibrary.SetInputMode_UIOnlyEx` _returnvalue _returnvalue_2) ; stops player from moving in screen
    (set `PlayerController.bShowMouseCursor` true _returnvalue)
    (`self.SetActorHiddenInGame` (`GameplayStatics.GetPlayerCharacter` 0) true) ; optional to make player hidden
    (`KismetSystemLibrary.Delay` 3.0)
    (`SkeletalMeshComponent.PlayAnimation` (`self.SkeletalMeshGumball`) "/Game/BluePrints/Assets/GumBall/GumballMachineAnimVersion_Anim.GumballMachineAnimVersion_Anim" true)
    ;;[0 0.1328 1] sounds & animations
    (`KismetSystemLibrary.Delay` 1.0)
    (`GameplayStatics.PlaySound2D` null 1.0 1.0 0.0 null null)
    (`SkeletalMeshComponent.Stop` (`self.SkeletalMeshGumball`))))

(event `self.GumballBox.OnComponentBeginOverlap`
  (params (OverlappedComponent :type "PrimitiveComponent Object Reference") (OtherActor :type "Actor Object Reference") (OtherComp :type "PrimitiveComponent Object Reference") (OtherBodyIndex :type Integer) (bFromSweep :type Boolean) (SweepResult :type "HitResult Structure (by ref)"))
  ;[1 1 1] Interaction Window
  (cast `/Game/BluePrints/Characters/CharactBlueprints/ThirdPersonCharacter` OtherActor)
  (`self.EnableInput` (`GameplayStatics.GetPlayerController` 0)))

(event `self.GumballBox.OnComponentEndOverlap`
  (params (OverlappedComponent :type "PrimitiveComponent Object Reference") (OtherActor :type "Actor Object Reference") (OtherComp :type "PrimitiveComponent Object Reference") (OtherBodyIndex :type Integer))
  ;[1 1 1] Interaction Window
  (cast `/Game/BluePrints/Characters/CharactBlueprints/ThirdPersonCharacter` OtherActor)
  (`self.DisableInput` (`GameplayStatics.GetPlayerController` 0)))

(event `Key|F`
  (params (Key :type "Key Structure")))

(fn `UserConstructionScript`)