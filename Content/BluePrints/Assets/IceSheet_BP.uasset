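; IceSheet_BP is an ice sheet that slides the ThirdPersonCharacter across to its opposite end.
; Entering LeftBox or RightBox targets the opposite marker and, guarded by IsOnIce and a shared DoOnce, records the capsule's location.
; The MovePlayer timeline then lerps the actor there with a swept SetActorLocation, resetting both guards on finish.
; Impulse and spark-emitter logic is left disconnected.
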(event `self.ReceiveTick`
  (params (DeltaSeconds :type "Float (single-precision)")))

(event `self.leftBox.OnComponentBeginOverlap`
  (params (OverlappedComponent :type "PrimitiveComponent Object Reference") (OtherActor :type "Actor Object Reference") (OtherComp :type "PrimitiveComponent Object Reference") (OtherBodyIndex :type Integer) (bFromSweep :type Boolean) (SweepResult :type "HitResult Structure (by ref)"))
  (bind _asthird_person_character (cast `/Game/BluePrints/Characters/CharactBlueprints/ThirdPersonCharacter` OtherActor))
  (set `self.As Third Person Character` _asthird_person_character)
  (if (not (`self.isOnIce`))
    (set `self.isOnIce` true)
    (set `self.endLocation` (`SceneComponent.K2_GetComponentLocation` (`self.right`)))
    (`/Engine/EditorBlueprintResources/StandardMacros.DoOnce` false :!label _label
      (:`Completed`
        (set `self.locationStamp` (`SceneComponent.K2_GetComponentLocation` (`Character.CapsuleComponent` (`self.As Third Person Character`))))
        (bind (_direction _alpha) (`Timeline|MovePlayer` :!via `PlayFromStart`)
          (:`Update`
            (`self.K2_SetActorLocation` (`self.As Third Person Character`) (`KismetMathLibrary.VLerp` (`self.locationStamp`) (`self.endLocation`) _alpha) true false))
          (:`Finished`
            (set `self.isOnIce` false)
            (goto _label :!via `Reset`)))))))

(event `self.leftBox.OnComponentEndOverlap`
  (params (OverlappedComponent :type "PrimitiveComponent Object Reference") (OtherActor :type "Actor Object Reference") (OtherComp :type "PrimitiveComponent Object Reference") (OtherBodyIndex :type Integer))
  (bind _asthird_person_character (cast `/Game/BluePrints/Characters/CharactBlueprints/ThirdPersonCharacter` OtherActor))
  (set `self.As Third Person Character` _asthird_person_character) ; sets charcter reference back to null
)

(event `self.rightBox.OnComponentBeginOverlap`
  (params (OverlappedComponent :type "PrimitiveComponent Object Reference") (OtherActor :type "Actor Object Reference") (OtherComp :type "PrimitiveComponent Object Reference") (OtherBodyIndex :type Integer) (bFromSweep :type Boolean) (SweepResult :type "HitResult Structure (by ref)"))
  (bind _asthird_person_character (cast `/Game/BluePrints/Characters/CharactBlueprints/ThirdPersonCharacter` OtherActor))
  (set `self.As Third Person Character` _asthird_person_character)
  (if (not (`self.isOnIce`))
    (set `self.isOnIce` true)
    (set `self.endLocation` (`SceneComponent.K2_GetComponentLocation` (`self.left`)))
    (goto _label)))

(event `self.rightBox.OnComponentEndOverlap`
  (params (OverlappedComponent :type "PrimitiveComponent Object Reference") (OtherActor :type "Actor Object Reference") (OtherComp :type "PrimitiveComponent Object Reference") (OtherBodyIndex :type Integer))
  (bind _asthird_person_character (cast `/Game/BluePrints/Characters/CharactBlueprints/ThirdPersonCharacter` OtherActor))
  (set `self.As Third Person Character` _asthird_person_character) ; sets charcter reference back to null
)

(fn `UserConstructionScript`)