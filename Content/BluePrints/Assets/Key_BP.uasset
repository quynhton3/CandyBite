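; Key_BP is a scarf pickup that sets HasScarfP on the ThirdPersonCharacter that touches it.
; Overlapping ScarfBox sets the flag, waits briefly, spawns Niagara burst and flash effects at the pickup's location, the flash at a fixed height, then destroys the actor.
; A bob-and-rotate timeline and several scarf visibility nodes are left disconnected and never run.
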(event `self.ReceiveBeginPlay`)

(event `self.ReceiveActorBeginOverlap`
  (params (OtherActor :type "Actor Object Reference")))

(event `self.ScarfBox.OnComponentBeginOverlap`
  (params (OverlappedComponent :type "PrimitiveComponent Object Reference") (OtherActor :type "Actor Object Reference") (OtherComp :type "PrimitiveComponent Object Reference") (OtherBodyIndex :type Integer) (bFromSweep :type Boolean) (SweepResult :type "HitResult Structure (by ref)"))
  (bind (_returnvalue_x _returnvalue_y) (`KismetMathLibrary.BreakVector` (`self.K2_GetActorLocation`)))
  (bind _asthird_person_character (cast `/Game/BluePrints/Characters/CharactBlueprints/ThirdPersonCharacter` OtherActor))
  (set `/Game/BluePrints/Characters/CharactBlueprints/ThirdPersonCharacter.hasScarfP ` true _asthird_person_character)
  (`KismetSystemLibrary.Delay` 0.15)
  (`NiagaraFunctionLibrary.SpawnSystemAtLocation` "/Game/Particles/Niagaras/NS_Pickup_Burst.NS_Pickup_Burst" (`self.K2_GetActorLocation`))
  (`NiagaraFunctionLibrary.SpawnSystemAtLocation` "/Game/Particles/Niagaras/NS_Flash.NS_Flash" (`KismetMathLibrary.MakeVector` _returnvalue_x _returnvalue_y 200.0))
  (`self.K2_DestroyActor`))

(fn `UserConstructionScript`)