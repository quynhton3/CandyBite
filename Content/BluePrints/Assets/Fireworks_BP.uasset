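; Fireworks actor that launches a single Niagara firework effect at its own location.
; On BeginPlay it waits a random 15 to 30 seconds, then spawns the Hearts system once.
; An unconnected branch would randomly pick between Hearts, Brocade and Ring effects, but it never runs, so only Hearts appears.
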(event `self.ReceiveBeginPlay`
  (`KismetSystemLibrary.Delay` (`KismetMathLibrary.RandomFloatInRange` 15.0 30.0))
  ;[0 0 0] Firework 1
  (`NiagaraFunctionLibrary.SpawnSystemAtLocation` "/Game/VFX/Niagaras/NS_Firework_Hearts1.NS_Firework_Hearts1" (`self.K2_GetActorLocation`)))

(event `self.ReceiveTick`
  (params (DeltaSeconds :type "Float (single-precision)")))

(fn `UserConstructionScript`)