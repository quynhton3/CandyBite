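; Gingerbread destructible actor that breaks loose after repeated hits from the third-person character.
; Each character hit on the Destructible component increments the IsStacked3 counter until it reaches three.
; Later hits enable physics simulation and apply small radial damage at the impact point, with the character as damage causer.
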(event `self.Destructible.OnComponentHit`
  (params (HitComponent :type "PrimitiveComponent Object Reference") (OtherActor :type "Actor Object Reference") (OtherComp :type "PrimitiveComponent Object Reference") (NormalImpulse :type "Vector Structure") (Hit :type "HitResult Structure (by ref)"))
  (bind _asthird_person_character (cast `/Game/BluePrints/Characters/CharactBlueprints/ThirdPersonCharacter` OtherActor))
  (if (>= (`self.isStacked3?`) 3.0)
    (`PrimitiveComponent.SetSimulatePhysics` (`self.Destructible`) true)
    (`GameplayStatics.ApplyRadialDamage` :`BaseDamage` 10.0 :`Origin` (`.ImpactPoint` (`GameplayStatics.BreakHitResult` Hit)) :`DamageRadius` 60.0 :`DamageTypeClass` "/Script/Engine.DamageType" :`DamageCauser` _asthird_person_character :`InstigatedByController` null :`bDoFullDamage` true)
    (else
      (set `self.isStacked3?` (+ (`self.isStacked3?`) 1.0)))))

(fn `UserConstructionScript`)