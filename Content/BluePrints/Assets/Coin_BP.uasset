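; Coin pickup actor that is collected when a ThirdPersonCharacter overlaps its BoxCoin component.
; Collection increments the character's NumCoins, shows a new CoinAmount_WD widget, spawns a starburst particle and destroys the coin.
; A wormPawn overlap joins the same logic, but still writes to the ThirdPersonCharacter cast result rather than the worm.
; The Animator timeline for bobbing and spinning is present but never runs.
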(event `self.BoxCoin.OnComponentBeginOverlap`
  (params (OverlappedComponent :type "PrimitiveComponent Object Reference") (OtherActor :type "Actor Object Reference") (OtherComp :type "PrimitiveComponent Object Reference") (OtherBodyIndex :type Integer) (bFromSweep :type Boolean) (SweepResult :type "HitResult Structure (by ref)"))
  ;[1 1 1] coin added
  (`|ExecutionSequence`
    (:`then_0`
      (bind _asthird_person_character (cast `/Game/BluePrints/Characters/CharactBlueprints/ThirdPersonCharacter` OtherActor)))
    (:`then_1`
      (cast `/Game/BluePrints/Characters/CharactBlueprints/wormPawn` OtherActor) ; Shout out to Seabasssssssssssssssss
    ))
  (bind _returnvalue (+ (`/Game/BluePrints/Characters/CharactBlueprints/ThirdPersonCharacter.numCoins` _asthird_person_character) 1))
  (set `/Game/BluePrints/Characters/CharactBlueprints/ThirdPersonCharacter.numCoins` _returnvalue _asthird_person_character)
  (bind _returnvalue_2 (`|CreateWidget` "/Game/BluePrints/UI/coinAmount_WD.coinAmount_WD_C" null _returnvalue))
  (`UserWidget.AddToViewport` _returnvalue_2 0)
  (`GameplayStatics.SpawnEmitterAtLocation` "/Game/Particles/Particles/StarBurst2_CPS.StarBurst2_CPS" (`self.K2_GetActorLocation`))
  (`self.K2_DestroyActor`))

(event `self.BoxCoin.OnComponentEndOverlap`
  (params (OverlappedComponent :type "PrimitiveComponent Object Reference") (OtherActor :type "Actor Object Reference") (OtherComp :type "PrimitiveComponent Object Reference") (OtherBodyIndex :type Integer)))

(fn `UserConstructionScript`)