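; Candy-themed puzzle light that the player cycles through red, orange and blue with E while inside its overlap box.
; Each press updates the point light and candy cane through SwitchColor, then compares the index to LightOrderNumber.
; It reports to LightPuzzle_BP via AddTo on a match and RemoveFrom on a mismatch, the latter gated by a DoOnce that matches reset.
; BeginPlay colors the other candy meshes by the target number.
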(event `self.Box.OnComponentBeginOverlap`
  (params (OverlappedComponent :type "PrimitiveComponent Object Reference") (OtherActor :type "Actor Object Reference") (OtherComp :type "PrimitiveComponent Object Reference") (OtherBodyIndex :type Integer) (bFromSweep :type Boolean) (SweepResult :type "HitResult Structure (by ref)"))
  ;[1 1 1] Enable / Disable Input
  (`self.EnableInput` (`GameplayStatics.GetPlayerController` 0))
  (`/Game/BluePrints/Characters/CharactBlueprints/ThirdPersonCharacter.interact` (`self.Player REF`)))

(event `self.Box.OnComponentEndOverlap`
  (params (OverlappedComponent :type "PrimitiveComponent Object Reference") (OtherActor :type "Actor Object Reference") (OtherComp :type "PrimitiveComponent Object Reference") (OtherBodyIndex :type Integer))
  ;[1 1 1] Enable / Disable Input
  (`self.DisableInput` (`GameplayStatics.GetPlayerController` 0)))

(event `RemoveTo`
  (`/Engine/EditorBlueprintResources/StandardMacros.DoOnce` false :!label _label
    (:`Completed`
      (`/Game/BluePrints/Assets/LightPuzzle_BP.RemoveFrom` (`self.Puzzle`)))))

(event `Key|E`
  (params (Key :type "Key Structure"))
  (bind _lightint (`self.LightInt`))
  (bind _returnvalue (+ (`self.LightInt`) 1))
  ;[1 1 1] Interacted with
  (:`Pressed`
    (set `self.LightInt` _returnvalue) ; increases
    (if (== _returnvalue 4)
      (set `self.LightInt` 0) ; Resets it back to 0 if over
    )
    (`self.SwitchColor` _lightint)
    (if (== _lightint (`self.LightOrderNumber`))
      (`/Game/BluePrints/Assets/LightPuzzle_BP.AddTo` (`self.Puzzle`))
      (goto _label :!via `Reset`)
      (else
        (`self.RemoveTo`)))))

(event `self.ReceiveBeginPlay`
  (set `self.Player REF` (cast `/Game/BluePrints/Characters/CharactBlueprints/ThirdPersonCharacter` (`GameplayStatics.GetPlayerCharacter` 0) :!pure true))
  (bind _outactors (`GameplayStatics.GetAllActorsOfClass` "/Game/BluePrints/Assets/LightPuzzle_BP.LightPuzzle_BP_C"))
  (set `self.Puzzle` (`|GetArrayItem` _outactors)) ; setting instantiate
  (`|ExecutionSequence`
    (:`then_0`
      ;[1 1 1] Mesh Candy Cane Color
      (if (== (`self.LightOrderNumber`) 0)
        (`PrimitiveComponent.SetMaterial` (`self.CandyCaneMesh`) 0 "/Game/DECOR/FBXs/Materials/CandyCane_Red.CandyCane_Red")
        (`PrimitiveComponent.SetMaterial` (`self.GumDropMesh`) 0 "/Game/DECOR/FBXs/Materials/Gumdrop_Red.Gumdrop_Red")
        (`PrimitiveComponent.SetMaterial` (`self.smarty`) 0 "/Game/DECOR/FBXs/Materials/Pink_Smartie.Pink_Smartie")
        (`PrimitiveComponent.SetMaterial` (`self.smarty1`) 0 "/Game/DECOR/FBXs/Materials/Pink_Smartie.Pink_Smartie")))
    (:`then_1`
      (if (== (`self.LightOrderNumber`) 1)
        (`PrimitiveComponent.SetMaterial` (`self.CandyCaneMesh`) 0 "/Game/DECOR/FBXs/Materials/CandyCane_Orange.CandyCane_Orange")
        (`PrimitiveComponent.SetMaterial` (`self.GumDropMesh`) 0 "/Game/DECOR/FBXs/Materials/Gumdrop_Orange.Gumdrop_Orange")
        (`PrimitiveComponent.SetMaterial` (`self.smarty`) 0 "/Game/DECOR/FBXs/Materials/Blue_Smartie.Blue_Smartie")
        (`PrimitiveComponent.SetMaterial` (`self.smarty1`) 0 "/Game/DECOR/FBXs/Materials/Blue_Smartie.Blue_Smartie")))
    (:`then_2`
      (if (== (`self.LightOrderNumber`) 2)
        (`PrimitiveComponent.SetMaterial` (`self.CandyCaneMesh`) 0 "/Game/DECOR/FBXs/Materials/CandyCane_Blue.CandyCane_Blue")
        (`PrimitiveComponent.SetMaterial` (`self.GumDropMesh`) 0 "/Game/DECOR/FBXs/Materials/Gumdrop_Blue.Gumdrop_Blue")
        (`PrimitiveComponent.SetMaterial` (`self.smarty`) 0 "/Game/DECOR/FBXs/Materials/Blue_Smartie.Blue_Smartie")
        (`PrimitiveComponent.SetMaterial` (`self.smarty1`) 0 "/Game/DECOR/FBXs/Materials/Blue_Smartie.Blue_Smartie")))))

(fn `SwitchColor`
  (params (LightInt :type Integer))
  (bind _pointlight (`self.PointLight`))
  (bind _candycanemesh1 (`self.CandyCaneMesh1`))
  ;[1 1 1] Switch colors based on int
  (switch `int` LightInt
    (:`0`
      (`LightComponent.SetLightColor` _pointlight (struct :`R` 1.0 :`A` 1.0) true)
      (`PrimitiveComponent.SetMaterial` _candycanemesh1 0 "/Game/DECOR/FBXs/Materials/CandyCane_Red.CandyCane_Red"))
    (:`1`
      (`LightComponent.SetLightColor` _pointlight (struct :`R` 1.0 :`G` 0.50901 :`A` 1.0) true)
      (`PrimitiveComponent.SetMaterial` _candycanemesh1 0 "/Game/DECOR/FBXs/Materials/CandyCane_Orange.CandyCane_Orange"))
    (:`2`
      (`LightComponent.SetLightColor` _pointlight (struct :`G` 0.741678 :`B` 1.0 :`A` 1.0) true)
      (`PrimitiveComponent.SetMaterial` _candycanemesh1 0 "/Game/DECOR/FBXs/Materials/CandyCane_Blue.CandyCane_Blue"))))

(fn `UserConstructionScript`
  ;[1 1 1] Around 3 m
  (`self.SwitchColor` (`self.LightInt`)))