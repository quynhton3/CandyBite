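; Light puzzle manager Blueprint that opens the way once every Light_BP actor in the level has been counted.
; AddTo and RemoveFrom adjust an integer counter, which is kept from dropping below zero.
; When AddTo makes the count equal the number of Light_BP actors, WinningCondition plays the Winner timeline, which shifts the GingerBread component along Z each update to act as the opening door.
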(event `AddTo`
  ;[1 1 1] add until int == the  amount of lights are in the scene
  (set `self.Int` (+ (`self.Int`) 1))
  (bind _outactors (`GameplayStatics.GetAllActorsOfClass` "/Game/BluePrints/Assets/Light_BP.Light_BP_C"))
  (if (== (`KismetArrayLibrary.Array_Length` _outactors) (`self.Int`))
    (`self.WinningCondition`)))

(event `RemoveFrom`
  (bind _int (`self.Int`))
  ;[1 1 1] take Away Int
  (if (> _int 0)
    (set `self.Int` (- _int 1))))

(event `WinningCondition`
  ;[1 1 1] Opens Door
  (bind (_direction _newtrack_0) (`Timeline|Winner`)
    (:`Update`
      (`SceneComponent.K2_AddRelativeLocation` (`self.GingerBread`) (`KismetMathLibrary.MakeVector` 0.0 0.0 _newtrack_0) false false))))

(event `self.ReceiveTick`
  (params (DeltaSeconds :type "Float (single-precision)")))

(fn `UserConstructionScript`)