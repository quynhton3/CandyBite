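; IceCreamInselberg is a zone actor that shows a Frost HUD widget while the ThirdPersonCharacter overlaps its Box.
; The first overlap creates the widget through a DoOnce; later overlaps only toggle its visibility.
; The IsInIceCreamInselberg flag is set true only on that first entry and cleared on exit.
; Frost drain, reset and health damage logic exists but is disconnected and never runs.
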(event `self.ReceiveBeginPlay`)

(event `self.ReceiveTick`
  (params (DeltaSeconds :type "Float (single-precision)")))

(event `self.Box.OnComponentBeginOverlap`
  (params (OverlappedComponent :type "PrimitiveComponent Object Reference") (OtherActor :type "Actor Object Reference") (OtherComp :type "PrimitiveComponent Object Reference") (OtherBodyIndex :type Integer) (bFromSweep :type Boolean) (SweepResult :type "HitResult Structure (by ref)"))
  ;[1 1 1] Show
  (cast `/Game/BluePrints/Characters/CharactBlueprints/ThirdPersonCharacter` OtherActor)
  (`|ExecutionSequence`
    (:`then_0`
      (`/Engine/EditorBlueprintResources/StandardMacros.DoOnce` false ; else itll make a bunch
        (:`Completed`
          (bind _returnvalue (`|CreateWidget` "/Game/BluePrints/UI/Frost_WD.Frost_WD_C"))
          (bind _output_get (set `self.Frost WD REF` _returnvalue))
          (`UserWidget.AddToViewport` _output_get 0)
          (set `self.isInIceCreamInselberg` true))))
    (:`then_1`
      (`Widget.SetVisibility` (`self.Frost WD REF`) "Visible"))))

(event `self.Box.OnComponentEndOverlap`
  (params (OverlappedComponent :type "PrimitiveComponent Object Reference") (OtherActor :type "Actor Object Reference") (OtherComp :type "PrimitiveComponent Object Reference") (OtherBodyIndex :type Integer))
  ;[1 1 1] remove hud
  (cast `/Game/BluePrints/Characters/CharactBlueprints/ThirdPersonCharacter` OtherActor)
  (`/Engine/EditorBlueprintResources/StandardMacros.IsValid` (`self.Frost WD REF`)
    (:`Is Valid`
      (`Widget.SetVisibility` (`self.Frost WD REF`) "Hidden")
      (set `self.isInIceCreamInselberg` false))))

(fn `UserConstructionScript`)