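; Lever actor that requires holding Interact inside its box trigger for a per-instance duration, currently printing a placeholder message on completion.
; Player overlap enables input, shows a progress widget and opens a gate for the press.
; A retriggerable delay checks the hold flag at completion.
; In parallel, a timer's elapsed time feeds the widget through a recursive delay loop, which resets progress on release.
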(event `InputAction|Interact`
  (params (Key :type "Key Structure"))
  (:`Pressed`
    (set `self.isHeld?` true)
    (`/Engine/EditorBlueprintResources/StandardMacros.Gate` true :!label _label
      (:`Exit`
        (`|ExecutionSequence`
          (:`then_0`
            (`KismetSystemLibrary.RetriggerableDelay` (`self.Max Hold Time`)) ; 8m
            (if (`self.isHeld?`)
              (`KismetSystemLibrary.PrintString` "Hello")))
          (:`then_1`
            (`self.Timer`)
            (`self.Update Timer`))))))
  (:`Released`
    (set `self.isHeld?` false)))

(event `self.Box.OnComponentBeginOverlap`
  (params (OverlappedComponent :type "PrimitiveComponent Object Reference") (OtherActor :type "Actor Object Reference") (OtherComp :type "PrimitiveComponent Object Reference") (OtherBodyIndex :type Integer) (bFromSweep :type Boolean) (SweepResult :type "HitResult Structure (by ref)"))
  ;[1 1 1] Comment
  (cast `/Game/BluePrints/Characters/CharactBlueprints/ThirdPersonCharacter` OtherActor)
  (`self.EnableInput` (`GameplayStatics.GetPlayerController` 0))
  (bind _returnvalue (`|CreateWidget` "/Game/BluePrints/UI/Lever_WD.Lever_WD_C"))
  (bind _output_get (set `self.Lever WD REF` _returnvalue))
  (`UserWidget.AddToViewport` _output_get 0)
  (set `/Game/BluePrints/UI/Lever_WD.MaxTimeHeld` (`self.Max Hold Time`) _output_get)
  (goto _label :!via `Open`))

(event `self.Box.OnComponentEndOverlap`
  (params (OverlappedComponent :type "PrimitiveComponent Object Reference") (OtherActor :type "Actor Object Reference") (OtherComp :type "PrimitiveComponent Object Reference") (OtherBodyIndex :type Integer))
  ;[1 1 1] Comment
  (cast `/Game/BluePrints/Characters/CharactBlueprints/ThirdPersonCharacter` OtherActor)
  (`self.DisableInput` (`GameplayStatics.GetPlayerController` 0))
  (`Widget.RemoveFromParent` (stale `self.Box.OnComponentBeginOverlap` _returnvalue))
  (goto _label :!via `Close`))

(event `Stop Timer`
  ;[1 1 1] Timer (how long you have to hold it for to get the percentage go up and complete)
  (`KismetSystemLibrary.K2_PauseTimerHandle` (stale `Timer` _returnvalue)))

(event `Timer`
  ;[1 1 1] Timer (how long you have to hold it for to get the percentage go up and complete)
  (bind _returnvalue (`KismetSystemLibrary.K2_SetTimerDelegate` (delegate `Timer`) (`self.Max Hold Time`))))

(event `Update Timer`
  (bind _lever_wd_ref (`self.Lever WD REF`))
  ;[1 1 1] Timer (how long you have to hold it for to get the percentage go up and complete)
  (if (`self.isHeld?`)
    (set `/Game/BluePrints/UI/Lever_WD.TimeHeld` (`KismetSystemLibrary.K2_GetTimerElapsedTimeHandle` (stale `Timer` _returnvalue)) _lever_wd_ref)
    ;;[1 1 1] Constantly updates
    (`KismetSystemLibrary.Delay` 0.1)
    (`self.Update Timer`)
    (else
      (`self.Stop Timer`)
      (set `/Game/BluePrints/UI/Lever_WD.TimeHeld` 0.0 _lever_wd_ref))))

(fn `UserConstructionScript`)