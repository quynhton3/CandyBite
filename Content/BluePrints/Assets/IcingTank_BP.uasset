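; IcingTank_BP is an icing tank actor that the player fills with icing they carry.
; Its box overlap toggles actor input and an IcingTank_WD prompt widget for the ThirdPersonCharacter.
; Pressing E takes one NumIcing from the character, then increments CurrentIcingTank while below a hard-coded five.
; Reaching MaxIcingTank disables input and prints a debug message, though re-entering the box enables input again.
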(event `self.ReceiveBeginPlay`
  (bind _returnvalue (`|CreateWidget` "/Game/BluePrints/UI/MovementTutorial/IcingTank_WD.IcingTank_WD_C"))
  (set `self.tutorialRef` _returnvalue))

(event `Key|E`
  (params (Key :type "Key Structure"))
  ;[1 1 1] Filling tank up
  (:`Pressed`
    (bind _asthird_person_character (cast `/Game/BluePrints/Characters/CharactBlueprints/ThirdPersonCharacter` (`GameplayStatics.GetPlayerCharacter` 0)))
    (bind _numicing (`/Game/BluePrints/Characters/CharactBlueprints/ThirdPersonCharacter.numIcing` _asthird_person_character))
    (if (> _numicing 0)
      (set `/Game/BluePrints/Characters/CharactBlueprints/ThirdPersonCharacter.numIcing` (- _numicing 1) _asthird_person_character)
      (if (< (`self.currentIcingTank`) 5)
        (bind _output_get (set `self.currentIcingTank` (+ (`self.currentIcingTank`) 1)))
        (if (>= _output_get (`self.maxIcingTank`))
          (`self.DisableInput` (`GameplayStatics.GetPlayerController` 0))
          (`KismetSystemLibrary.PrintString` "Removed!"))))))

(event `self.Box.OnComponentBeginOverlap`
  (params (OverlappedComponent :type "PrimitiveComponent Object Reference") (OtherActor :type "Actor Object Reference") (OtherComp :type "PrimitiveComponent Object Reference") (OtherBodyIndex :type Integer) (bFromSweep :type Boolean) (SweepResult :type "HitResult Structure (by ref)"))
  ;[1 1 1] take User Input
  (cast `/Game/BluePrints/Characters/CharactBlueprints/ThirdPersonCharacter` OtherActor)
  (`self.EnableInput` (`GameplayStatics.GetPlayerController` 0))
  (`UserWidget.AddToViewport` (`self.tutorialRef`) 0))

(event `self.Box.OnComponentEndOverlap`
  (params (OverlappedComponent :type "PrimitiveComponent Object Reference") (OtherActor :type "Actor Object Reference") (OtherComp :type "PrimitiveComponent Object Reference") (OtherBodyIndex :type Integer))
  ;[1 1 1] take User Input
  (cast `/Game/BluePrints/Characters/CharactBlueprints/ThirdPersonCharacter` OtherActor)
  (`self.DisableInput` (`GameplayStatics.GetPlayerController` 0))
  (`Widget.RemoveFromParent` (`self.tutorialRef`)))

(fn `UserConstructionScript`)