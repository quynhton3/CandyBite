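; Mushroom enemy that chases the player, attacks at close range and destroys itself when its health runs out.
; Detection and attack-range overlap boxes set flags that Tick reads to drive AIMoveTo, face the player and run attacks.
; A delay-timed, flag-gated attack toggles the mushroom AnimBP and subtracts player HP directly, with no hit check at impact.
; Incoming damage spawns Niagara effects; the player's AttackEnemies dispatcher resets hit state.
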(event `self.ReceiveBeginPlay`
  (`|ExecutionSequence`
    (:`then_0`
      (`SceneComponent.K2_AttachToComponent` (`self.MushroomsAttackBox`) (`self.Mesh`) "RightHand" "KeepRelative" "KeepRelative" "KeepRelative" true))
    (:`then_1`
      ;[1 1 1] Hit once
      (bind _asthird_person_character (cast `/Game/BluePrints/Characters/CharactBlueprints/ThirdPersonCharacter` (`GameplayStatics.GetPlayerCharacter` 0)))
      (bind _output_get (set `self.charRef` _asthird_person_character))
      (add `/Game/BluePrints/Characters/CharactBlueprints/ThirdPersonCharacter.AttackEnemies` _output_get (delegate `ResetHit`)))
    (:`then_2`
      (bind _asmushroom_ab (cast `/Game/Character/Enemy/Mushroom/mushroom_AB` (`SkeletalMeshComponent.GetAnimInstance` (`self.Mesh`))))
      (set `self.As Mushroom AB` _asmushroom_ab))))

(event `ResetHit`
  ;[1 1 1] Hit once
  (set `self.isHit` false)
  ;[1 1 1] https://www.youtube.com/watch?v=SyGIpX8WzZk&ab_channel=JoshDoesCoding
  (set `self.hasBeenAttacked` true))

(event `self.ReceiveAnyDamage`
  (params (Damage :type "Float (single-precision)") (DamageType :type "DamageType Object Reference") (InstigatedBy :type "Controller Object Reference") (DamageCauser :type "Actor Object Reference"))
  (bind (_returnvalue_x _returnvalue_y _returnvalue_z) (`KismetMathLibrary.BreakVector` (`self.K2_GetActorLocation`)))
  ;[1 0.03103 0.05092] Takes Damage & Dying
  (set `self.enemyHealth` (- (`self.enemyHealth`) Damage))
  (`NiagaraFunctionLibrary.SpawnSystemAtLocation` "/Game/Particles/Niagaras/NS_PowEnemyDamaged.NS_PowEnemyDamaged" (`KismetMathLibrary.MakeVector` _returnvalue_x _returnvalue_y (+ _returnvalue_z 30.0)))
  (if (<= (`self.enemyHealth`) 0.0)
    (`self.K2_DestroyActor`)))

(event `self.ReceiveTick`
  (params (DeltaSeconds :type "Float (single-precision)"))
  (bind _charref (`self.charRef`))
  (`|ExecutionSequence`
    (:`then_0`
      ;[0.555 1 0.879] Chasing https://www.youtube.com/watch?v=Yl_mH8IgzC0&ab_channel=JoshDoesCoding
      (if (`self.hasDetectedPlayer`)
        (`|AIMoveTo` self (`self.K2_GetActorLocation` (`GameplayStatics.GetPlayerCharacter` 0)) null 20.0
          (:`then`
            (`SceneComponent.K2_SetWorldRotation` (`self.Mesh`) (`KismetMathLibrary.MakeRotator` 0.0 0.0 (+ (.yaw (`KismetMathLibrary.FindLookAtRotation` (`self.K2_GetActorLocation`) (`self.K2_GetActorLocation` (`GameplayStatics.GetPlayerCharacter` 0)))) 270.0)) false false)))))
    (:`then_1`
      ;[1 1 1] Scuffed Attacking player (Can scrap)
      (if (and (`self.canAttackPlayer`) (not (`self.IsAttackingPlayer`)))
        (set `self.IsAttackingPlayer` true)
        (set `/Game/Character/Enemy/Mushroom/mushroom_AB.isAttacking?` true (`self.As Mushroom AB`))
        (`KismetSystemLibrary.Delay` 0.5)
        (set `/Game/BluePrints/Characters/CharactBlueprints/ThirdPersonCharacter.CurrentHP` (- (`/Game/BluePrints/Characters/CharactBlueprints/ThirdPersonCharacter.CurrentHP` _charref) 10.0) _charref)
        (`NiagaraFunctionLibrary.SpawnSystemAtLocation` "/Game/Particles/Niagaras/NS_Coin_Burst.NS_Coin_Burst" (`self.K2_GetActorLocation` _charref))
        (`KismetSystemLibrary.Delay` 0.5)
        (set `/Game/Character/Enemy/Mushroom/mushroom_AB.isAttacking?` false (`self.As Mushroom AB`))
        (`KismetSystemLibrary.Delay` 2.0)
        (set `self.IsAttackingPlayer` false)))))

(event `self.MushroomsAttackRangeBox.OnComponentBeginOverlap`
  (params (OverlappedComponent :type "PrimitiveComponent Object Reference") (OtherActor :type "Actor Object Reference") (OtherComp :type "PrimitiveComponent Object Reference") (OtherBodyIndex :type Integer) (bFromSweep :type Boolean) (SweepResult :type "HitResult Structure (by ref)"))
  ;[1 0.507 0.1473] When player enters box, enemy attacks
  (if (`ActorComponent.ComponentHasTag` OtherComp "Player")
    (set `self.canAttackPlayer` true)))

(event `self.MushroomsAttackRangeBox.OnComponentEndOverlap`
  (params (OverlappedComponent :type "PrimitiveComponent Object Reference") (OtherActor :type "Actor Object Reference") (OtherComp :type "PrimitiveComponent Object Reference") (OtherBodyIndex :type Integer))
  ;[1 0.507 0.1473] When player enters box, enemy attacks
  (if (`ActorComponent.ComponentHasTag` OtherComp "Player")
    (set `self.canAttackPlayer` false)))

(event `self.MushroomDetectedPlayer.OnComponentBeginOverlap`
  (params (OverlappedComponent :type "PrimitiveComponent Object Reference") (OtherActor :type "Actor Object Reference") (OtherComp :type "PrimitiveComponent Object Reference") (OtherBodyIndex :type Integer) (bFromSweep :type Boolean) (SweepResult :type "HitResult Structure (by ref)"))
  ;[1 1 1] Detected Player
  (if (`ActorComponent.ComponentHasTag` OtherComp "Player")
    (set `self.hasDetectedPlayer` true)))

(event `self.MushroomDetectedPlayer.OnComponentEndOverlap`
  (params (OverlappedComponent :type "PrimitiveComponent Object Reference") (OtherActor :type "Actor Object Reference") (OtherComp :type "PrimitiveComponent Object Reference") (OtherBodyIndex :type Integer))
  ;[1 1 1] Detected Player
  (if (`ActorComponent.ComponentHasTag` OtherComp "Player")
    (set `self.hasDetectedPlayer` false)))

(fn `UserConstructionScript`)