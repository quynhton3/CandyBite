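; Attack system component for Enemy2 that handles a montage-based basic attack with combo buffering, triggered by the ability1 Attack input when CanAttack is set.
; BasicAttack saves input if already attacking, otherwise dispatches on AttackIndex.
; AttackCombo consumes saved input to re-enter that dispatch or calls StopCombo to reset.
; Only Attack1 exists, guarded by a DoOnce, and nothing here sets IsAttacking true.
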(event `Attack 1`
  ;[1 1 1] Attack 1
  (`/Engine/EditorBlueprintResources/StandardMacros.DoOnce` false :!label _label
    (:`Completed`
      (`KismetSystemLibrary.Delay` 0.1)
      (`|PlayMontage` null
        (:`then`
          (set `self.attack Index` 1)
          (goto _label :!via `Reset`))))))

(event `InputAction|ability1 Attack`
  (params (Key :type "Key Structure"))
  ;[1 0.5156 0.5156] Attack Input
  (:`Pressed`
    (if (`self.can Attack?`)
      (`self.Basic Attack`))))

(event `Key|LeftMouseButton`
  (params (Key :type "Key Structure"))
  ;[1 0.5156 0.5156] Attack Input
)

(event `Basic Attack`
  ;[1 0.5156 0.5156] Basic Attack
  (if (`self.is Attacking?`)
    (set `self.save Attack?` true) ; to transition for combos
    (else
      (set `self.save Attack?` false)
      (switch `int` (`self.attack Index`) :!label _label_2
        (:`0`
          (`self.Attack 1`))))))

(event `Attack Combo`
  ;[1 0.5156 0.5156] Combo Attack Continue
  (if (`self.save Attack?`)
    (set `self.save Attack?` false)
    (goto _label_2)
    (else
      (`self.Stop Combo `))))

(event `Stop Combo`
  ;[1 0.5156 0.5156] Stops Combos / Attacks
  (set `self.is Attacking?` false)
  (set `self.attack Index` 0))